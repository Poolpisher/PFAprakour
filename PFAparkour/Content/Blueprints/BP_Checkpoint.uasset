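; BP_Checkpoint is a checkpoint that saves its index and arrow transform to the game instance once its enemies are cleared, then destroys itself.
; On BeginPlay it briefly teleports away and back, and its box overlaps register melee enemies.
; A player overlap starts a Tick check of those enemies' validity.
; If its index matches the saved one on BeginPlay, it destroys equal- or higher-numbered checkpoints and their enemies.
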(event `self.ReceiveBeginPlay`
  (set `self.originalLocation` (`self.K2_GetActorLocation`))
  (`self.K2_SetActorLocation` (0.0 0.0 -10000.0))
  (`KismetSystemLibrary.Delay` 0.1)
  (`self.K2_SetActorLocation` (`self.originalLocation`))
  (bind _ascustom_game_instance (cast `/Game/CustomGameInstance` (`GameplayStatics.GetGameInstance`)))
  (if (== (`/Game/CustomGameInstance.checkPointIndex` _ascustom_game_instance) (`self.checkPointNumber`))
    (for _array_element (`self.enemies`)
      (`/Engine/EditorBlueprintResources/StandardMacros.IsValid` _array_element
        (:`Is Valid`
          (`self.K2_DestroyActor` _array_element))))
    (bind _outactors (`GameplayStatics.GetAllActorsOfClass` "BP_Checkpoint_C"))
    (for _array_element_2 _outactors
      (if (not (< (`/Game/Blueprints/BP_Checkpoint.checkPointNumber` _array_element_2) (`self.checkPointNumber`)))
        (for _array_element_3 (`/Game/Blueprints/BP_Checkpoint.enemies` _array_element_2)
          (`/Engine/EditorBlueprintResources/StandardMacros.IsValid` _array_element_3
            (:`Is Valid`
              (`self.K2_DestroyActor` _array_element_3))))
        (`self.K2_DestroyActor` _array_element_2)))
    (`self.K2_DestroyActor` :!label _label)))

(event `self.Box.OnComponentBeginOverlap`
  (params (OverlappedComponent :type "PrimitiveComponent Object Reference") (OtherActor :type "Actor Object Reference") (OtherComp :type "PrimitiveComponent Object Reference") (OtherBodyIndex :type Integer) (bFromSweep :type Boolean) (SweepResult :type "HitResult Structure (by ref)"))
  (cast `/Game/FirstPerson/Blueprints/BP_FirstPersonCharacter` OtherActor
    (:`then`
      (set `self.canCheckForEnemies` true))
    (:`CastFailed`
      (bind _asbp_enemy (cast `/Game/Blueprints/Enemies/BP_EnemyMelee` OtherActor))
      (`KismetArrayLibrary.Array_AddUnique` (`self.enemies`) _asbp_enemy))))

(event `SetCheckPoint`
  (bind _ascustom_game_instance (cast `/Game/CustomGameInstance` (`GameplayStatics.GetGameInstance`)))
  (set `/Game/CustomGameInstance.checkPointIndex` (`self.checkPointNumber`) _ascustom_game_instance)
  (set `/Game/CustomGameInstance.lastCheckPoint` (`SceneComponent.K2_GetComponentToWorld` (`self.Arrow`)) _ascustom_game_instance)
  (goto _label))

(event `self.ReceiveTick`
  (params (DeltaSeconds :type "Float (single-precision)"))
  (if (`self.canCheckForEnemies`)
    (for _array_element (`self.enemies`)
      (`/Engine/EditorBlueprintResources/StandardMacros.IsValid` _array_element
        (:`Is Valid`
          (set `self.canSetCheckPoint` false)
          (break))
        (:`Is Not Valid`
          (set `self.canSetCheckPoint` true))))
    (if (`self.canSetCheckPoint`)
      (`/Engine/EditorBlueprintResources/StandardMacros.DoOnce` false
        (:`Completed`
          (`self.SetCheckPoint`))))))

(fn `UserConstructionScript`)