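; BP_Objective is a placeable objective marker that chains level goals and shows each on the player's HUD.
; A first objective reveals its widget and posts its name and description to the first-person character's HUD shortly after BeginPlay.
; When the player overlaps its box, it reveals and posts the linked NewObjective, or removes the HUD objectives box if none is set, then destroys itself.
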(event `self.ReceiveBeginPlay`
  (`KismetSystemLibrary.Delay` 0.2)
  (if (`self.isFirstObjective`)
    (`SceneComponent.SetHiddenInGame` (`self.Widget`) false false)
    (bind _asbp_first_person_character (cast `/Game/FirstPerson/Blueprints/BP_FirstPersonCharacter` (`GameplayStatics.GetPlayerCharacter` 0)))
    (`/Game/Widget/W_Main.SetObjective` (`/Game/FirstPerson/Blueprints/BP_FirstPersonCharacter.mainHUD` _asbp_first_person_character) (`self.objectiveName`) (`self.objectiveDescription`))))

(event `self.Box.OnComponentBeginOverlap`
  (params (OverlappedComponent :type "PrimitiveComponent Object Reference") (OtherActor :type "Actor Object Reference") (OtherComp :type "PrimitiveComponent Object Reference") (OtherBodyIndex :type Integer) (bFromSweep :type Boolean) (SweepResult :type "HitResult Structure (by ref)"))
  (cast `/Game/FirstPerson/Blueprints/BP_FirstPersonCharacter` OtherActor)
  (`self.SetNewObjective`))

(event `SetNewObjective`
  (bind _newobjective (`self.newObjective`)
    (:`then`
      (`SceneComponent.SetHiddenInGame` (`/Game/Blueprints/BP_Objective.Widget` _newobjective) false false)
      (bind _asbp_first_person_character (cast `/Game/FirstPerson/Blueprints/BP_FirstPersonCharacter` (`GameplayStatics.GetPlayerCharacter` 0)))
      (`/Game/Widget/W_Main.SetObjective` (`/Game/FirstPerson/Blueprints/BP_FirstPersonCharacter.mainHUD` _asbp_first_person_character) (`/Game/Blueprints/BP_Objective.objectiveName` _newobjective) (`/Game/Blueprints/BP_Objective.objectiveDescription` _newobjective)))
    (:`else`
      (bind _asbp_first_person_character_2 (cast `/Game/FirstPerson/Blueprints/BP_FirstPersonCharacter` (`GameplayStatics.GetPlayerCharacter` 0)))
      (`Widget.RemoveFromParent` (`/Game/Widget/W_Main.HorizontalBox_Objectives` (`/Game/FirstPerson/Blueprints/BP_FirstPersonCharacter.mainHUD` _asbp_first_person_character_2)))))
  (`self.K2_DestroyActor`))

(fn `UserConstructionScript`)