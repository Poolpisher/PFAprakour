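; Enemy character whose EnemyType makes it a chasing melee Mover or a ranged Shooter, setting mesh and adding a shoot component.
; PawnSensing acquires the player to start AI chase or enable shooting; a per-tick line trace drops the target when blocked.
; Movers kill via box trace on arrival; body contact kills the player unless dashing or grappling, which instead kills the enemy and launches the player upward.
; GetTeleportLocation halts both characters and returns the EnemyBack transform.
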(event `self.ReceiveBeginPlay`
  (bind _mesh (`self.Mesh`))
  ;[0 0 0 1 34] Set enemy
  (switch `/Game/Blueprints/Enemies/Enum_EnemyType` (`self.enemyType`)
    (:`NewEnumerator1`
      (`SkeletalMeshComponent.SetSkeletalMeshAsset` _mesh "/Game/3D/melee_enemy_V2.melee_enemy_V2"))
    (:`NewEnumerator2`
      (`SkeletalMeshComponent.SetSkeletalMeshAsset` _mesh "/Game/Characters/Mannequins/Meshes/SKM_Manny.SKM_Manny")
      (`AddComponent|NODE_AddComp_EnemyShoot-0` :`range` (`self.shootRange`) :`cooldown` (`self.shootCD`)))))

(event `self.ReceiveTick`
  (params (DeltaSeconds :type "Float (single-precision)"))
  ;[0 0 0 1 34] Check if player is still in range
  (bind _playerref (`self.playerRef`)
    (:`then`
      (bind _outhit (`KismetSystemLibrary.LineTraceSingle` :`Start` (`self.K2_GetActorLocation`) :`End` (`self.K2_GetActorLocation` _playerref) :`TraceChannel` "TraceTypeQuery2" :`DrawTime` 0.2))
      (cast `/Game/FirstPerson/Blueprints/BP_FirstPersonCharacter` (`.HitActor` (`GameplayStatics.BreakHitResult` _outhit))
        (:`CastFailed`
          (set `self.canShoot` false)
          (`MovementComponent.StopMovementImmediately` (`self.CharacterMovement`))
          (set `self.playerRef` null))))
    (:`else`)))

(event `self.CapsuleComponent.OnComponentBeginOverlap`
  (params (OverlappedComponent :type "PrimitiveComponent Object Reference") (OtherActor :type "Actor Object Reference") (OtherComp :type "PrimitiveComponent Object Reference") (OtherBodyIndex :type Integer) (bFromSweep :type Boolean) (SweepResult :type "HitResult Structure (by ref)"))
  ;[1 1 0 1 34] On player overlap
  (bind _asbp_first_person_character (cast `/Game/FirstPerson/Blueprints/BP_FirstPersonCharacter` OtherActor))
  (if (or (`/Game/FirstPerson/Blueprints/BP_FirstPersonCharacter.isInDash` _asbp_first_person_character) (`/Game/FirstPerson/Blueprints/BP_FirstPersonCharacter.hasGrappled` _asbp_first_person_character))
    (`/Game/FirstPerson/Blueprints/BP_FirstPersonCharacter.SetInvicibilityFrames` _asbp_first_person_character)
    (bind _charactermovement (`Character.CharacterMovement` _asbp_first_person_character))
    (bind (_velocity_x _velocity_y) (`KismetMathLibrary.BreakVector` (`MovementComponent.Velocity` _charactermovement)))
    (set `MovementComponent.Velocity` (`KismetMathLibrary.MakeVector` (/ _velocity_x 5.0) (/ _velocity_y 5.0)) _charactermovement)
    (set `/Game/FirstPerson/Blueprints/BP_FirstPersonCharacter.isInDash` false _asbp_first_person_character)
    (`self.LaunchCharacter` _asbp_first_person_character (0.0 0.0 2000.0) false true)
    (`self.SetDeath`)
    (else
      (`/Game/FirstPerson/Blueprints/BP_FirstPersonCharacter.SetDeath` _asbp_first_person_character))))

(event `/Game/Blueprints/Enemies/Interface_Enemy.GetAttack`
  ;[1 0 0 1 34] Get attack/Death
  (`self.SetDeath`))

(event `SetDeath`
  ;[1 0 0 1 34] Get attack/Death
  (`GameplayStatics.PlaySound2D` "/Game/Audio/SFX/Enemies/S_EnemyDeath.S_EnemyDeath" 1.0 1.0 0.0 null null)
  (`self.K2_DestroyActor`))

(event `Chase`
  (params (TargetActor :type "Actor Object Reference"))
  (bind _returnvalue (`SceneComponent.K2_GetComponentLocation` (`self.ActorForward`)))
  ;[0 0 1 1 34] Chase player
  (`|AIMoveTo` (`PawnMovementComponent.GetPawnOwner` (`self.CharacterMovement`)) (0.0 0.0 0.0) TargetActor 150.0 true
    (:`OnSuccess`
      (`KismetSystemLibrary.Delay` 0.2)
      (bind _outhits (`KismetSystemLibrary.BoxTraceMulti` _returnvalue _returnvalue (100.0 200.0 100.0) (struct) "TraceTypeQuery2"))
      (for _array_element _outhits
        (bind _asbp_first_person_character (cast `/Game/FirstPerson/Blueprints/BP_FirstPersonCharacter` (`.HitActor` (`GameplayStatics.BreakHitResult` _array_element))))
        (`/Game/FirstPerson/Blueprints/BP_FirstPersonCharacter.SetDeath` _asbp_first_person_character)
        (break)))))

(event `self.PawnSensing.OnSeePawn`
  (params (Pawn :type "Pawn Object Reference"))
  ;[0 1 0 1 34] On player seen
  (bind _asbp_first_person_character (cast `/Game/FirstPerson/Blueprints/BP_FirstPersonCharacter` Pawn))
  (bind _output_get (set `self.playerRef` _asbp_first_person_character))
  (switch `/Game/Blueprints/Enemies/Enum_EnemyType` (`self.enemyType`)
    (:`NewEnumerator1`
      (`self.Chase` _output_get))
    (:`NewEnumerator2`
      (set `self.canShoot` true))))

(fn `GetTeleportLocation`
  (returns (EnemyBack :type "Transform Structure"))
  (`MovementComponent.StopMovementImmediately` (`self.CharacterMovement`))
  (set `self.canShoot` false)
  (bind _asbp_first_person_character (cast `/Game/FirstPerson/Blueprints/BP_FirstPersonCharacter` (`GameplayStatics.GetPlayerCharacter` 0)))
  (set `MovementComponent.Velocity` (0.0 0.0 0.0) (`Character.CharacterMovement` _asbp_first_person_character))
  (return (`SceneComponent.K2_GetComponentToWorld` (`self.EnemyBack`))))

(fn `UserConstructionScript`
  (bind _mesh (`self.Mesh`))
  (switch `/Game/Blueprints/Enemies/Enum_EnemyType` (`self.enemyType`)
    (:`NewEnumerator1`
      (`SkeletalMeshComponent.SetSkeletalMeshAsset` _mesh "/Game/3D/melee_enemy_V2.melee_enemy_V2"))
    (:`NewEnumerator2`
      (`SkeletalMeshComponent.SetSkeletalMeshAsset` _mesh "/Game/Characters/Mannequins/Meshes/SKM_Manny.SKM_Manny"))))