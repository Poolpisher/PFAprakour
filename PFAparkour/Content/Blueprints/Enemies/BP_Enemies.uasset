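; Enemy actor that dies in one hit and kills the first-person player on contact unless the player is dashing.
; A capsule overlap during a dash ends the dash, launches the player upward and destroys the enemy.
; BeginPlay adds a shooting component for the Shooter enemy type.
; GetAttack also destroys the enemy, and GetTeleportLocation exposes the EnemyBack transform as a teleport target.
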(event `self.ReceiveBeginPlay`
  (switch `/Game/Blueprints/Enemies/Enum_EnemyType` (`self.enemyType`)
    (:`NewEnumerator2`
      (`AddComponent|NODE_AddComp_EnemyShoot-0`))))

(event `self.CapsuleComponent.OnComponentBeginOverlap`
  (params (OverlappedComponent :type "PrimitiveComponent Object Reference") (OtherActor :type "Actor Object Reference") (OtherComp :type "PrimitiveComponent Object Reference") (OtherBodyIndex :type Integer) (bFromSweep :type Boolean) (SweepResult :type "HitResult Structure (by ref)"))
  (bind _asbp_first_person_character (cast `/Game/FirstPerson/Blueprints/BP_FirstPersonCharacter` OtherActor))
  (if (`/Game/FirstPerson/Blueprints/BP_FirstPersonCharacter.isInDash` _asbp_first_person_character)
    (set `/Game/FirstPerson/Blueprints/BP_FirstPersonCharacter.isInDash` false _asbp_first_person_character)
    (`self.LaunchCharacter` _asbp_first_person_character (0.0 0.0 1000.0) false false)
    (`self.SetDeath`)
    (else
      (`/Game/FirstPerson/Blueprints/BP_FirstPersonCharacter.SetDeath` _asbp_first_person_character))))

(event `SetDeath`
  (`self.K2_DestroyActor`))

(event `/Game/Blueprints/Enemies/Interface_Enemy.GetAttack`
  (`self.SetDeath`))

(fn `GetTeleportLocation`
  (returns (EnemyBack :type "Transform Structure"))
  (return (`SceneComponent.K2_GetComponentToWorld` (`self.EnemyBack`))))

(fn `UserConstructionScript`)