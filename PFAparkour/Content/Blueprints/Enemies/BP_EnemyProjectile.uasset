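; Enemy projectile that charges while attached, then detaches after a fixed delay, aims once at the player and flies straight.
; Tick moves it forward by Speed per frame, unscaled by delta time, and destroys it after a set lifetime.
; Overlap kills the player unless countering, when it is destroyed or, if the game instance allows deflection, turned toward its instigator.
; Deflected shots can kill melee enemies.
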(event `self.ReceiveTick`
  (params (DeltaSeconds :type "Float (single-precision)"))
  (bind _autodestroytimer (`self.AutoDestroyTimer`))
  (if (`self.isLaunched`)
    (`self.K2_SetActorLocation` (+ (`self.K2_GetActorLocation`) (* (`KismetMathLibrary.GetForwardVector` (`self.K2_GetActorRotation`)) (`self.Speed`))))
    (if (> _autodestroytimer 8.0)
      (`self.K2_DestroyActor`)
      (else
        (set `self.AutoDestroyTimer` (+ _autodestroytimer DeltaSeconds))))))

(event `self.ReceiveBeginPlay`
  (`KismetSystemLibrary.Delay` 3.2)
  (bind _asbp_first_person_character (cast `/Game/FirstPerson/Blueprints/BP_FirstPersonCharacter` (`GameplayStatics.GetPlayerCharacter` 0)))
  (`self.K2_SetActorRotation` (`KismetMathLibrary.FindLookAtRotation` (`self.K2_GetActorLocation`) (`self.K2_GetActorLocation` _asbp_first_person_character)))
  (`ActorComponent.SetActive` (`self.Projectile_VFX`) true true)
  (`ActorComponent.SetActive` (`self.ProjectileConstruction`) false false)
  (`SceneComponent.K2_DetachFromComponent` (`self.DefaultSceneRoot`) "KeepWorld" "KeepWorld" "KeepWorld" true)
  (set `self.isLaunched` true)
  (`KismetSystemLibrary.Delay` 20.0)
  (`self.K2_DestroyActor`))

(event `self.SphereCollision.OnComponentBeginOverlap`
  (params (OverlappedComponent :type "PrimitiveComponent Object Reference") (OtherActor :type "Actor Object Reference") (OtherComp :type "PrimitiveComponent Object Reference") (OtherBodyIndex :type Integer) (bFromSweep :type Boolean) (SweepResult :type "HitResult Structure (by ref)"))
  (if (`self.isLaunched`)
    (bind _asbp_first_person_character (cast `/Game/FirstPerson/Blueprints/BP_FirstPersonCharacter` OtherActor)
      (:`then`
        (if (`/Game/FirstPerson/Blueprints/BP_FirstPersonCharacter.isCountering` _asbp_first_person_character)
          (`self.Counter`)
          (else
            (`/Game/FirstPerson/Blueprints/BP_FirstPersonCharacter.SetDeath` _asbp_first_person_character)
            (`self.K2_DestroyActor` :!label _label))))
      (:`CastFailed`
        (bind _asbp_enemy_melee (cast `/Game/Blueprints/Enemies/BP_EnemyMelee` OtherActor))
        (if (`self.isCountered`)
          (`/Game/Blueprints/Enemies/BP_EnemyMelee.SetDeath` _asbp_enemy_melee)
          (goto _label))))))

(event `Counter`
  (if (`self.isLaunched`)
    (bind _ascustom_game_instance (cast `/Game/CustomGameInstance` (`GameplayStatics.GetGameInstance`)))
    (if (`/Game/CustomGameInstance.deflectBullet` _ascustom_game_instance)
      (set `self.isCountered` true)
      (`self.K2_SetActorRotation` (`KismetMathLibrary.FindLookAtRotation` (`self.K2_GetActorLocation`) (`self.K2_GetActorLocation` (`self.GetInstigator`))))
      (`GameplayStatics.PlaySound2D` "/Game/Audio/SFX/Capacity/Counter/Cue_Counter.Cue_Counter" 1.0 1.0 0.0 null null)
      (else
        (`self.K2_DestroyActor`)))))

(fn `UserConstructionScript`)