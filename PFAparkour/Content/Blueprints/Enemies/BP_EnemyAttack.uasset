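; BP_EnemyAttack is an enemy that chases the first-person player on sight and kills them on contact.
; PawnSensing starts an AI MoveTo toward the player, and either reaching them or a capsule overlap triggers the player's death.
; An overlap during a dash or grapple instead launches the player upward, grants invisibility frames and destroys the enemy.
; GetAttack also destroys it, while GetTeleportLocation halts its movement and returns the EnemyBack transform.
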(event `self.CapsuleComponent.OnComponentBeginOverlap`
  (params (OverlappedComponent :type "PrimitiveComponent Object Reference") (OtherActor :type "Actor Object Reference") (OtherComp :type "PrimitiveComponent Object Reference") (OtherBodyIndex :type Integer) (bFromSweep :type Boolean) (SweepResult :type "HitResult Structure (by ref)"))
  (bind _asbp_first_person_character (cast `/Game/FirstPerson/Blueprints/BP_FirstPersonCharacter` OtherActor))
  (if (or (`/Game/FirstPerson/Blueprints/BP_FirstPersonCharacter.isInDash` _asbp_first_person_character) (`/Game/FirstPerson/Blueprints/BP_FirstPersonCharacter.isGrappling` _asbp_first_person_character))
    (set `/Game/FirstPerson/Blueprints/BP_FirstPersonCharacter.isInDash` false _asbp_first_person_character)
    (`self.LaunchCharacter` _asbp_first_person_character (0.0 0.0 1000.0) false false)
    (`/Game/FirstPerson/Blueprints/BP_FirstPersonCharacter.SetInvisibilityFrames` _asbp_first_person_character)
    (`self.SetDeath`)
    (else
      (`/Game/FirstPerson/Blueprints/BP_FirstPersonCharacter.SetDeath` _asbp_first_person_character))))

(event `/Game/Blueprints/Enemies/Interface_Enemy.GetAttack`
  (`self.SetDeath`))

(event `SetDeath`
  (`self.K2_DestroyActor`))

(event `self.PawnSensing.OnSeePawn`
  (params (Pawn :type "Pawn Object Reference"))
  (bind _asbp_first_person_character (cast `/Game/FirstPerson/Blueprints/BP_FirstPersonCharacter` Pawn))
  (`self.Chase` _asbp_first_person_character))

(event `Chase`
  (params (TargetActor :type "Actor Object Reference"))
  (`|AIMoveTo` (`PawnMovementComponent.GetPawnOwner` (`self.CharacterMovement`)) (0.0 0.0 0.0) TargetActor
    (:`OnSuccess`
      (bind _asbp_first_person_character (cast `/Game/FirstPerson/Blueprints/BP_FirstPersonCharacter` TargetActor))
      (`/Game/FirstPerson/Blueprints/BP_FirstPersonCharacter.SetDeath` _asbp_first_person_character))))

(fn `GetTeleportLocation`
  (returns (EnemyBack :type "Transform Structure"))
  (`MovementComponent.StopMovementImmediately` (`self.CharacterMovement`))
  (return (`SceneComponent.K2_GetComponentToWorld` (`self.EnemyBack`))))

(fn `UserConstructionScript`)