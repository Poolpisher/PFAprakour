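; Enemy shooting component that lets a BP_EnemyMelee owner fire projectiles at the first-person player.
; Each Tick, if the player is within Range and the owner's CanShoot is set, it turns the enemy's yaw toward the player.
; A DoOnce reset after a Cooldown delay gates firing.
; Each shot spawns BP_EnemyProjectile at the owner's ActorForward transform, attaches it to the enemy mesh and plays a 2D sound.
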(event `self.ReceiveTick`
  (params (DeltaSeconds :type "Float (single-precision)"))
  (bind _returnvalue (`Actor.K2_GetActorLocation` (`self.GetOwner`)))
  (bind _asbp_first_person_character (cast `/Game/FirstPerson/Blueprints/BP_FirstPersonCharacter` (`GameplayStatics.GetPlayerCharacter` 0)))
  (bind _asbp_enemy_melee (cast `/Game/Blueprints/Enemies/BP_EnemyMelee` (`self.GetOwner`)))
  (bind _returnvalue_2 (`Actor.K2_GetActorLocation` _asbp_first_person_character))
  (if (and (< (`KismetMathLibrary.Vector_Distance` _returnvalue_2 _returnvalue) (`self.range`)) (`/Game/Blueprints/Enemies/BP_EnemyMelee.canShoot` _asbp_enemy_melee))
    (bind (_returnvalue_roll _returnvalue_pitch _returnvalue_yaw) (`KismetMathLibrary.BreakRotator` (`KismetMathLibrary.FindLookAtRotation` _returnvalue_2 _returnvalue)))
    (`Actor.K2_SetActorRotation` _asbp_enemy_melee (`KismetMathLibrary.MakeRotator` 0.0 0.0 (- _returnvalue_yaw 180.0)) false)
    (`/Engine/EditorBlueprintResources/StandardMacros.DoOnce` false :!label _label
      (:`Completed`
        (bind _asbp_enemy_melee_2 (cast `/Game/Blueprints/Enemies/BP_EnemyMelee` (`self.GetOwner`)))
        (bind _returnvalue_3 (`|SpawnActorFromClass` "/Game/Blueprints/Enemies/BP_EnemyProjectile.BP_EnemyProjectile_C" (`SceneComponent.K2_GetComponentToWorld` (`/Game/Blueprints/Enemies/BP_EnemyMelee.ActorForward` _asbp_enemy_melee_2)) "Undefined" "MultiplyWithRoot" null _asbp_enemy_melee_2))
        (bind _output_get (set `self.projectileRef` _returnvalue_3))
        (`Actor.K2_AttachToComponent` _output_get (`Character.Mesh` _asbp_enemy_melee_2) "None" "KeepWorld" "KeepWorld" "KeepWorld" true)
        (`GameplayStatics.PlaySound2D` "/Game/Audio/SFX/Enemies/Projectiles/Cue_Projectile.Cue_Projectile" 1.0 1.0 0.0 null null)
        (`KismetSystemLibrary.Delay` (`self.cooldown`))
        (goto _label :!via `Reset`)))))