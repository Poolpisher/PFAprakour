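; BP_PortalResource is a pickup that refreshes the first-person player's movement abilities on overlap.
; It re-enables grapple, clears the dash state, refills move capacity, updates the HUD and plays a bonus sound.
; It then hides itself and disables collision, resetting a DoOnce.
; Tick fires that DoOnce while the player is moving on the ground, so the pickup reappears once the player is grounded.
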(event `self.Box.OnComponentBeginOverlap`
  (params (OverlappedComponent :type "PrimitiveComponent Object Reference") (OtherActor :type "Actor Object Reference") (OtherComp :type "PrimitiveComponent Object Reference") (OtherBodyIndex :type Integer) (bFromSweep :type Boolean) (SweepResult :type "HitResult Structure (by ref)"))
  (bind _asbp_first_person_character (cast `/Game/FirstPerson/Blueprints/BP_FirstPersonCharacter` OtherActor))
  (`GameplayStatics.PlaySound2D` "/Game/Audio/SFX/LevelElements/Portal/S_PortalBonus.S_PortalBonus" 1.0 1.0 0.0 null null)
  (set `/Game/FirstPerson/Blueprints/BP_FirstPersonCharacter.canUseGrapple` true _asbp_first_person_character)
  (set `/Game/FirstPerson/Blueprints/BP_FirstPersonCharacter.isInDash` false _asbp_first_person_character)
  (set `/Game/FirstPerson/Blueprints/BP_FirstPersonCharacter.currentMoveCapacity` (`/Game/FirstPerson/Blueprints/BP_FirstPersonCharacter.maxMoveCapacity` _asbp_first_person_character) _asbp_first_person_character)
  (`/Game/Widget/W_Main.UpdateMovementPoints` (`/Game/FirstPerson/Blueprints/BP_FirstPersonCharacter.mainHUD` _asbp_first_person_character))
  (`SceneComponent.SetHiddenInGame` (`self.Cube11`) true true)
  (`PrimitiveComponent.SetCollisionEnabled` (`self.Box`) "NoCollision")
  (goto _label :!via `Reset`))

(event `self.ReceiveTick`
  (params (DeltaSeconds :type "Float (single-precision)"))
  (bind _asbp_first_person_character (cast `/Game/FirstPerson/Blueprints/BP_FirstPersonCharacter` (`GameplayStatics.GetPlayerCharacter` 0)))
  (if (`NavMovementComponent.IsMovingOnGround` (`Character.CharacterMovement` _asbp_first_person_character))
    (`/Engine/EditorBlueprintResources/StandardMacros.DoOnce` false :!label _label
      (:`Completed`
        (`SceneComponent.SetHiddenInGame` (`self.Cube11`) false true)
        (`PrimitiveComponent.SetCollisionEnabled` (`self.Box`) "QueryOnly")))))

(fn `UserConstructionScript`)