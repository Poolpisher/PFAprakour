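; BP_Platform is a placeable platform with a normal mode and a bounce mode.
; A flip-flop toggles the mode, swapping the cube's material between preview and placed variants.
; Finishing creation applies the final material, enables collision and starts a short timed self-destruct.
; In bounce mode, hits from the first-person character launch it with a Z override and play a bounce sound.
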(event `StartCheckToDestroy`
  (set `self.hasBeenPlaced` true)
  (`KismetSystemLibrary.Delay` 5.0)
  (`self.K2_DestroyActor`))

(event `ChangePlatformMode`
  (params (isCreatingPlatform :type Boolean))
  (bind _cube (`self.Cube`))
  (bind _isa (`/Engine/EditorBlueprintResources/StandardMacros.FlipFlop`)
    (:`A`
      _)
    (:`B`
      _))
  (bind _output_get (set `self.isBounceMod` _isa))
  (if _output_get
    (`PrimitiveComponent.SetMaterial` _cube 0 (select `bool` isCreatingPlatform :`false` "/Game/Materials/M_TestBouncePlatform.M_TestBouncePlatform" :`true` "/Game/Materials/M_TestBouncePlatformToPlace.M_TestBouncePlatformToPlace" :!type "MaterialInterface Object Reference"))
    (else
      (`PrimitiveComponent.SetMaterial` _cube 0 (select `bool` isCreatingPlatform :`false` "/Game/Materials/M_TestPlatform.M_TestPlatform" :`true` "/Game/Materials/M_TestPlatformToPlace.M_TestPlatformToPlace" :!type "MaterialInterface Object Reference")))))

(event `FinishCreatePlatform`
  (bind _cube (`self.Cube`))
  (`PrimitiveComponent.SetMaterial` _cube 0 (select `bool` (`self.isBounceMod`) :`false` "/Game/Materials/M_TestPlatform.M_TestPlatform" :`true` "/Game/Materials/M_TestBouncePlatform.M_TestBouncePlatform" :!type "MaterialInterface Object Reference"))
  (`PrimitiveComponent.SetCollisionEnabled` _cube "QueryAndPhysics")
  (`self.StartCheckToDestroy`))

(event `self.Cube.OnComponentHit`
  (params (HitComponent :type "PrimitiveComponent Object Reference") (OtherActor :type "Actor Object Reference") (OtherComp :type "PrimitiveComponent Object Reference") (NormalImpulse :type "Vector Structure") (Hit :type "HitResult Structure (by ref)"))
  (if (`self.isBounceMod`)
    (bind _asbp_first_person_character (cast `/Game/FirstPerson/Blueprints/BP_FirstPersonCharacter` OtherActor))
    (`Character.LaunchCharacter` _asbp_first_person_character (`self.launchVelocity`) false true)
    (`GameplayStatics.PlaySoundAtLocation` "/Game/Audio/SFX/LevelElements/Bumper/S_Bounce.S_Bounce" (`self.K2_GetActorLocation`) (struct) 1.0 1.0 0.0 null null null null)))

(fn `UserConstructionScript`
  (if (not (`self.isSpawned`))
    (`PrimitiveComponent.SetMaterial` (`self.Cube`) 0 (select `bool` (`self.isBounceMod`) :`false` "/Game/Materials/M_TestPlatform.M_TestPlatform" :`true` "/Game/Materials/M_TestBouncePlatform.M_TestBouncePlatform" :!type "MaterialInterface Object Reference"))))