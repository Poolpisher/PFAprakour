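; One-shot portal trigger that moves the first-person player to a new set of level actors.
; On BeginPlay it hides every actor in Levels, keeping the destination invisible until the portal is used.
; When the player overlaps the box, it reveals Levels and destroys everything in LevelsToHide.
; It then zeroes velocity, teleports the player to PlayerSpawn's transform, applies yaw and forward input, and destroys itself.
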(event `self.ReceiveBeginPlay`
  (for _array_element (`self.levels`)
    (`self.SetActorHiddenInGame` _array_element true)))

(event `self.Box.OnComponentBeginOverlap`
  (params (OverlappedComponent :type "PrimitiveComponent Object Reference") (OtherActor :type "Actor Object Reference") (OtherComp :type "PrimitiveComponent Object Reference") (OtherBodyIndex :type Integer) (bFromSweep :type Boolean) (SweepResult :type "HitResult Structure (by ref)"))
  (bind _asbp_first_person_character (cast `/Game/FirstPerson/Blueprints/BP_FirstPersonCharacter` OtherActor))
  (for _array_element (`self.levels`)
    (`self.SetActorHiddenInGame` _array_element false))
  (for _array_element_2 (`self.levelsToHide`)
    (`self.K2_DestroyActor` _array_element_2))
  (set `MovementComponent.Velocity` (0.0 0.0 0.0) (`Character.CharacterMovement` _asbp_first_person_character))
  (`self.K2_SetActorTransform` _asbp_first_person_character (`self.GetTransform` (`self.playerSpawn`)) false true)
  (`Pawn.AddControllerYawInput` _asbp_first_person_character 360.0)
  (`Pawn.AddMovementInput` _asbp_first_person_character (`self.GetActorForwardVector` _asbp_first_person_character) 1.0 false)
  (`self.K2_DestroyActor`))

(fn `UserConstructionScript`)