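; BP_PlatformReveal is a platform that toggles between a solid revealed state and a to-be-placed state that pawns pass through.
; Reveal stores the state, swaps the cube's material and switches Pawn collision between Block and Ignore, while Camera collision always blocks.
; BeginPlay applies the initial state, and SetPlatform flips it with a 2D sound.
; The construction script previews the matching material in the editor.
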(event `self.ReceiveBeginPlay`
  (`self.Reveal` (`self.isRevealed`)))

(event `Reveal`
  (params (newReveal :type Boolean))
  (bind _cube (`self.Cube`))
  (bind _output_get (set `self.isRevealed` newReveal))
  (`PrimitiveComponent.SetMaterial` _cube 0 (select `bool` _output_get :`false` "/Game/Materials/M_TestPlatformToPlace.M_TestPlatformToPlace" :`true` "/Game/Materials/M_TestPlatform.M_TestPlatform" :!type "MaterialInterface Object Reference"))
  (`PrimitiveComponent.SetCollisionResponseToChannel` _cube "ECC_Pawn" (select `bool` _output_get :`false` "ECR_Ignore" :`true` "ECR_Block" :!type "ECollisionResponse Enum"))
  (`PrimitiveComponent.SetCollisionResponseToChannel` _cube "ECC_Camera" "ECR_Block"))

(event `/Game/Blueprints/Interface_Platform.SetPlatform`
  (bind _returnvalue (not (`self.isRevealed`)))
  (`self.Reveal` _returnvalue)
  (`GameplayStatics.PlaySound2D` (select `bool` _returnvalue :`false` "/Game/Audio/SFX/LevelElements/Platform/S_UnrevealPlatform.S_UnrevealPlatform" :`true` "/Game/Audio/SFX/LevelElements/Platform/S_RevealPlatform.S_RevealPlatform" :!type "SoundBase Object Reference") 1.0 1.0 0.0 null null))

(fn `UserConstructionScript`
  (`PrimitiveComponent.SetMaterial` (`self.Cube`) 0 (select `bool` (`self.isRevealed`) :`false` "/Game/Materials/M_TestPlatformToPlace.M_TestPlatformToPlace" :`true` "/Game/Materials/M_TestPlatform.M_TestPlatform" :!type "MaterialInterface Object Reference")))