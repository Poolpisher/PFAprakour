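; Enemy projectile that aims at the first-person player on spawn and can be deflected back at its shooter.
; Tick moves it along its forward vector by a per-frame speed, without sweep or delta time.
; Sphere overlap kills a non-countering player; a countering one triggers Counter, which destroys the projectile or, if the GameInstance allows deflection, turns it toward its Instigator.
; Once countered, it kills any enemy shooter it touches.
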(event `self.ReceiveTick`
  (params (DeltaSeconds :type "Float (single-precision)"))
  (`self.K2_SetActorLocation` (+ (`self.K2_GetActorLocation`) (* (`KismetMathLibrary.GetForwardVector` (`self.K2_GetActorRotation`)) (`self.Speed`)))))

(event `self.ReceiveBeginPlay`
  (bind _asbp_first_person_character (cast `/Game/FirstPerson/Blueprints/BP_FirstPersonCharacter` (`GameplayStatics.GetPlayerCharacter` 0)))
  (`self.K2_SetActorRotation` (`KismetMathLibrary.FindLookAtRotation` (`self.K2_GetActorLocation`) (`self.K2_GetActorLocation` _asbp_first_person_character))))

(event `self.Sphere.OnComponentBeginOverlap`
  (params (OverlappedComponent :type "PrimitiveComponent Object Reference") (OtherActor :type "Actor Object Reference") (OtherComp :type "PrimitiveComponent Object Reference") (OtherBodyIndex :type Integer) (bFromSweep :type Boolean) (SweepResult :type "HitResult Structure (by ref)"))
  (bind _asbp_first_person_character (cast `/Game/FirstPerson/Blueprints/BP_FirstPersonCharacter` OtherActor)
    (:`then`
      (if (`/Game/FirstPerson/Blueprints/BP_FirstPersonCharacter.isCounter` _asbp_first_person_character)
        (`self.Counter`)
        (else
          (`/Game/FirstPerson/Blueprints/BP_FirstPersonCharacter.SetDeath` _asbp_first_person_character)
          (`self.K2_DestroyActor` :!label _label))))
    (:`CastFailed`
      (bind _asbp_enemy_shooter (cast `/Game/Blueprints/BP_EnemyShooter` OtherActor))
      (if (`self.isCountered`)
        (`/Game/Blueprints/BP_EnemyShooter.SetDeath` _asbp_enemy_shooter)
        (goto _label)))))

(event `Counter`
  (bind _ascustom_game_instance (cast `/Game/CustomGameInstance` (`GameplayStatics.GetGameInstance`)))
  (if (`/Game/CustomGameInstance.deflectBullet` _ascustom_game_instance)
    (set `self.isCountered` true)
    (`self.K2_SetActorRotation` (`KismetMathLibrary.FindLookAtRotation` (`self.K2_GetActorLocation`) (`self.K2_GetActorLocation` (`self.GetInstigator`))))
    (else
      (`self.K2_DestroyActor`))))

(fn `UserConstructionScript`)