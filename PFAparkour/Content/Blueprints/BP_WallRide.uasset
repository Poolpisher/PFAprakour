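; Wall-ride surface actor that lets the first-person player run along it while overlapping its box.
; On entry it stops grappling, switches movement to Flying with Z velocity zeroed each tick, and loops a ride sound.
; Traces determine wall side and travel direction between begin and end markers, feeding arm animation, forward vector and camera roll.
; On exit it resets player state, eases roll back via timelines and restores Falling after a short delay.
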(event `WallRideSounds`
  (`GameplayStatics.PlaySound2D` "/Game/Audio/SFX/LevelElements/WallRide/Cue_WallRide.Cue_WallRide" 1.0 1.0 0.0 null null))

(event `self.Box.OnComponentBeginOverlap`
  (params (OverlappedComponent :type "PrimitiveComponent Object Reference") (OtherActor :type "Actor Object Reference") (OtherComp :type "PrimitiveComponent Object Reference") (OtherBodyIndex :type Integer) (bFromSweep :type Boolean) (SweepResult :type "HitResult Structure (by ref)"))
  (bind _asbp_first_person_character (cast `/Game/FirstPerson/Blueprints/BP_FirstPersonCharacter` OtherActor))
  (bind _returnvalue (`KismetSystemLibrary.K2_SetTimerDelegate` (delegate `WallRideSounds`) 0.15 true))
  (set `self.soundsEvent` _returnvalue)
  (set `/Game/FirstPerson/Blueprints/BP_FirstPersonCharacter.wallRideRef` self _asbp_first_person_character)
  (bind _output_get (set `self.playerRef` _asbp_first_person_character))
  (`/Game/FirstPerson/Blueprints/BP_FirstPersonCharacter.StopGraplin` _output_get)
  (bind _out_hit_trace_end (`self.Linetrace_PlayerForward` 20000.0))
  (bind _output_get_2 (set `self.distancePlayerforwardBegin` (`KismetMathLibrary.Vector_Distance` _out_hit_trace_end (`SceneComponent.K2_GetComponentLocation` (`self.WallBegin`)))))
  (bind _output_get_3 (set `self.distancePlayerforwardEnd` (`KismetMathLibrary.Vector_Distance` _out_hit_trace_end (`SceneComponent.K2_GetComponentLocation` (`self.WallEnd`)))))
  (set `self.isComingFromTheBegining` (select `bool` (<= _output_get_2 _output_get_3) :`false` true))
  (set `/Game/FirstPerson/Blueprints/BP_FirstPersonCharacter.moveLeftRightMultiplier` 0.0 _output_get)
  (set `/Game/FirstPerson/Blueprints/BP_FirstPersonCharacter.isWallRiding` true _output_get)
  (set `/Game/FirstPerson/Blueprints/BP_FirstPersonCharacter.enumAnim` "NewEnumerator2" _output_get)
  (bind _charactermovement (`Character.CharacterMovement` _output_get))
  (bind (_returnvalue_x _returnvalue_y) (`KismetMathLibrary.BreakVector` (/ (`MovementComponent.Velocity` _charactermovement) 1)))
  (set `MovementComponent.Velocity` (`KismetMathLibrary.MakeVector` _returnvalue_x _returnvalue_y) _charactermovement)
  (`CharacterMovementComponent.SetMovementMode` _charactermovement "MOVE_Flying" 0)
  (`self.SetCameraView`))

(event `self.Box.OnComponentEndOverlap`
  (params (OverlappedComponent :type "PrimitiveComponent Object Reference") (OtherActor :type "Actor Object Reference") (OtherComp :type "PrimitiveComponent Object Reference") (OtherBodyIndex :type Integer))
  (bind _returnvalue (`GameplayStatics.GetPlayerController` 0))
  (bind _returnvalue_2 (`GameplayStatics.GetPlayerController` 0))
  (bind (_returnvalue_roll _returnvalue_pitch _returnvalue_yaw) (`KismetMathLibrary.BreakRotator` (`Controller.GetControlRotation` _returnvalue)))
  (bind (_returnvalue_roll_2 _returnvalue_pitch_2 _returnvalue_yaw_2) (`KismetMathLibrary.BreakRotator` (`Controller.GetControlRotation` (`GameplayStatics.GetPlayerController` 0))))
  (bind (_returnvalue_roll_3 _returnvalue_pitch_3 _returnvalue_yaw_3) (`KismetMathLibrary.BreakRotator` (`Controller.GetControlRotation` _returnvalue_2)))
  (bind _asbp_first_person_character (cast `/Game/FirstPerson/Blueprints/BP_FirstPersonCharacter` OtherActor))
  (`KismetSystemLibrary.K2_ClearAndInvalidateTimerHandle` (`self.soundsEvent`))
  (set `self.playerRef` null)
  (if (== (`/Game/FirstPerson/Blueprints/BP_FirstPersonCharacter.wallRideRef` _asbp_first_person_character) self)
    (set `/Game/FirstPerson/Blueprints/BP_FirstPersonCharacter.isInDash` false _asbp_first_person_character)
    (set `/Game/FirstPerson/Blueprints/BP_FirstPersonCharacter.moveLeftRightMultiplier` 1.0 _asbp_first_person_character)
    (set `/Game/FirstPerson/Blueprints/BP_FirstPersonCharacter.isWallRiding` false _asbp_first_person_character)
    (if (!= _returnvalue_roll_2 0.0)
      (bind _output_get (set `self.targetNoramlView` (+ _returnvalue_roll_2 (select `bool` (`self.isOnLeft`) :`false` -25.0 :`true` 25.0 :!type "Float (single-precision)"))))
      (if (`TimelineComponent.IsPlaying` (`self.Timeline_StartWallRide`))
        (`|ExecutionSequence`
          (:`then_0`
            (bind (_direction _newtrack_0) (`Timeline|Timeline_StartWallRide` :!via `Reverse` :!label _label)
              (:`Update`
                (`Controller.SetControlRotation` _returnvalue_2 (`KismetMathLibrary.MakeRotator` (`KismetMathLibrary.Lerp` (stale `SetCameraView` _output_get_2) (+ (stale `SetCameraView` _output_get_2) (select `bool` (stale `SetCameraView` _output_get) :`false` 25.0 :`true` -25.0 :!type "Float (single-precision)")) _newtrack_0) _returnvalue_pitch_3 _returnvalue_yaw_3)))
              (:`Finished`
                (goto _label_3 :!via `Reset`))))
          (:`then_1`
            (`/Game/FirstPerson/Blueprints/BP_FirstPersonCharacter.ResetWallRideJump` _asbp_first_person_character :!label _label_2)
            (`Controller.SetControlRotation` _returnvalue (`KismetMathLibrary.MakeRotator` 0.0 _returnvalue_pitch _returnvalue_yaw))
            (`KismetSystemLibrary.Delay` 0.2)
            (bind _charactermovement (`Character.CharacterMovement` _asbp_first_person_character))
            (if (`|EnumEquality` (`CharacterMovementComponent.MovementMode` _charactermovement) "MOVE_Flying")
              (`CharacterMovementComponent.SetMovementMode` _charactermovement "MOVE_Falling" 0))))
        (else
          (bind (_direction_2 _newtrack_0_2) (`Timeline|Timeline_EndWallRide` :!via `PlayFromStart`)
            (:`Update`
              (`Controller.SetControlRotation` _returnvalue (`KismetMathLibrary.MakeRotator` (`KismetMathLibrary.Lerp` _returnvalue_roll_2 _output_get _newtrack_0_2) _returnvalue_pitch_2 _returnvalue_yaw_2)))
            (:`Finished`
              (goto _label_2)))))
      (else
        (goto _label_2)))))

(event `DeactiveCollision`
  (`PrimitiveComponent.SetCollisionEnabled` (`self.Box`) "NoCollision")
  (`PrimitiveComponent.SetCollisionEnabled` (`self.Cube`) "NoCollision")
  (`KismetSystemLibrary.Delay` 0.2)
  (`PrimitiveComponent.SetCollisionEnabled` (`self.Box`) "QueryOnly")
  (`PrimitiveComponent.SetCollisionEnabled` (`self.Cube`) "QueryOnly"))

(event `SetCameraView`
  (bind _returnvalue (`GameplayStatics.GetPlayerController` 0))
  (bind _iscomingfromthebegining (`self.isComingFromTheBegining`))
  (bind _returnvalue_2 (`SceneComponent.GetForwardVector` (`self.RightForwardRef`)))
  (bind _returnvalue_3 (`SceneComponent.GetForwardVector` (`self.LeftForwardRef`)))
  (bind (_returnvalue_roll _returnvalue_pitch _returnvalue_yaw) (`KismetMathLibrary.BreakRotator` (`Controller.GetControlRotation` _returnvalue)))
  (bind _returnvalue_roll_2 (`KismetMathLibrary.BreakRotator` (`Controller.GetControlRotation` (`GameplayStatics.GetPlayerController` 0))))
  (bind (_out_hit_blocking_hit _out_hit_hit_actor) (`self.Linetrace` 400.0))
  (bind _output_get (set `self.isOnLeft` (and _out_hit_blocking_hit (== _out_hit_hit_actor self))))
  (bind _asbp_first_person_character (cast `/Game/FirstPerson/Blueprints/BP_FirstPersonCharacter` (`GameplayStatics.GetPlayerCharacter` 0)))
  (bind _asabp_character_arms (cast `/Game/FirstPersonArms/ParkourCharacter/MainCharacter/ABP_CharacterArms` (`SkeletalMeshComponent.GetAnimInstance` (`/Game/FirstPerson/Blueprints/BP_FirstPersonCharacter.FirstPersonMesh` _asbp_first_person_character))))
  (set `/Game/FirstPersonArms/ParkourCharacter/MainCharacter/ABP_CharacterArms.IsRightWallRun` _output_get _asabp_character_arms)
  (set `/Game/FirstPerson/Blueprints/BP_FirstPersonCharacter.wallRideForward` (select `bool` _output_get :`false` (select `bool` _iscomingfromthebegining :`false` _returnvalue_3 :`true` _returnvalue_2) :`true` (select `bool` _iscomingfromthebegining :`false` _returnvalue_3 :`true` _returnvalue_2)) _asbp_first_person_character)
  (if (or (> _returnvalue_roll_2 359.0) (< _returnvalue_roll_2 1.0))
    (`Controller.SetControlRotation` _returnvalue (`KismetMathLibrary.MakeRotator` 0.0 _returnvalue_pitch _returnvalue_yaw))
    (`/Engine/EditorBlueprintResources/StandardMacros.DoOnce` false :!label _label_3
      (:`Completed`
        (bind _output_get_2 (set `self.orginalCameraXrot` _returnvalue_roll))
        (goto _label :!via `PlayFromStart`)))))

(event `self.ReceiveTick`
  (params (DeltaSeconds :type "Float (single-precision)"))
  (bind _playerref (`self.playerRef`)
    (:`then`
      (bind (_returnvalue_x _returnvalue_y) (`KismetMathLibrary.BreakVector` (`self.GetVelocity` _playerref)))
      (set `MovementComponent.Velocity` (`KismetMathLibrary.MakeVector` _returnvalue_x _returnvalue_y) (`Character.CharacterMovement` _playerref)))
    (:`else`)))

(fn `GetIsOnRight`
  (returns (Value :type "Float (double-precision)"))
  (bind _returnvalue (`self.K2_GetActorLocation` (`self.playerRef`)))
  (return (`KismetMathLibrary.SelectFloat` -1.0 1.0 (> (`KismetMathLibrary.VSize` (- (`SceneComponent.K2_GetComponentLocation` (`self.RightForwardRef`)) _returnvalue)) (`KismetMathLibrary.VSize` (- (`SceneComponent.K2_GetComponentLocation` (`self.LeftForwardRef`)) _returnvalue))))))

(fn `Linetrace`
  (params (length :type "Float (double-precision)" :default 300.0) (DrawDebugType :type "EDrawDebugTrace Enum" :default "None"))
  (returns (`Out Hit Blocking Hit` :type Boolean) (`Out Hit Hit Actor` :type "Actor Object Reference") (`Out Hit Trace Start` :type "Vector Structure"))
  (bind _asbp_first_person_character (cast `/Game/FirstPerson/Blueprints/BP_FirstPersonCharacter` (`GameplayStatics.GetPlayerCharacter` 0)))
  (bind _returnvalue (`self.K2_GetActorLocation` _asbp_first_person_character))
  (bind _outhit (`KismetSystemLibrary.LineTraceSingle` _returnvalue (+ _returnvalue (* (`KismetMathLibrary.Normal` (- (`self.GetActorForwardVector` _asbp_first_person_character) (* (`self.GetActorRightVector` _asbp_first_person_character) -1))) length)) "TraceTypeQuery2" false (`|MakeArray` _asbp_first_person_character :!type "Actor Object Reference") DrawDebugType false))
  (return (`GameplayStatics.BreakHitResult` _outhit) (`.HitActor` (`GameplayStatics.BreakHitResult` _outhit)) (`.TraceStart` (`GameplayStatics.BreakHitResult` _outhit))))

(fn `Linetrace_PlayerForward`
  (params (length :type "Float (double-precision)" :default 20000.0) (DrawDebugType :type "EDrawDebugTrace Enum" :default "None"))
  (returns (`Out Hit Trace End` :type "Vector Structure"))
  (bind _firstpersoncamera (`/Game/FirstPerson/Blueprints/BP_FirstPersonCharacter.FirstPersonCamera` (`self.playerRef`)))
  (bind _returnvalue (`SceneComponent.K2_GetComponentLocation` _firstpersoncamera))
  (bind _outhit (`KismetSystemLibrary.LineTraceSingle` :`Start` _returnvalue :`End` (+ _returnvalue (* (`SceneComponent.GetForwardVector` _firstpersoncamera) length)) :`TraceChannel` "TraceTypeQuery2" :`DrawDebugType` DrawDebugType :`DrawTime` 2.0))
  (return (`.TraceEnd` (`GameplayStatics.BreakHitResult` _outhit))))

(fn `UserConstructionScript`)