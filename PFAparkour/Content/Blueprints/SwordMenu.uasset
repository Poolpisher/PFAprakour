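; SwordMenu is a menu sword that animates its reveal material when the game is started from the menu.
; On BeginPlay it creates a dynamic instance of the character sword material, waits a tick, then binds to the StartGame dispatcher on the first top-level W_Menu widget.
; That event plays DisappearTimeline, which drives the SwordReveal scalar parameter, apparently to make the sword disappear.
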(event `self.ReceiveBeginPlay`
  (bind _returnvalue (`PrimitiveComponent.CreateDynamicMaterialInstance` (`self.SkeletalMeshComponent`) 0 "/Game/FirstPersonArms/ParkourCharacter/Sword/Textures/MI_CharacterSword.MI_CharacterSword" "None"))
  (set `self.SwordMat` _returnvalue)
  (`KismetSystemLibrary.DelayUntilNextTick`)
  (bind _foundwidgets (`WidgetBlueprintLibrary.GetAllWidgetsOfClass` "/Game/Widget/Menu/W_Menu.W_Menu_C"))
  (add `/Game/Widget/Menu/W_Menu.StartGame` (`|GetArrayItem` _foundwidgets) (delegate `StartGame_Event`)))

(event `StartGame_Event`
  (bind (_direction _lerpvalue) (`Timeline|DisappearTimeline` :!via `PlayFromStart`)
    (:`Update`
      (`MaterialInstanceDynamic.SetScalarParameterValue` (`self.SwordMat`) "SwordReveal" _lerpvalue))))

(fn `UserConstructionScript`)