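; BP_PlatformPieces is a platform in pieces that assembles when SetPlatform fires, once only, with a reveal sound.
; BeginPlay gathers four scene components into an array and speeds up the timeline.
; MovePlatform lerps each piece to SceneObjective's location while rotating its first child to zero world rotation.
; The timeline's Finished pin advances the index and calls MovePlatform again, so pieces move sequentially until no valid entry remains.
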(event `self.ReceiveBeginPlay`
  (set `self.scenesArray` (`|MakeArray` (`self.Scene`) (`self.Scene1`) (`self.Scene2`) (`self.Scene3`)))
  (`TimelineComponent.SetPlayRate` (`self.Timeline_SetPlatform`) 5.0))

(event `MovePlatform`
  (bind _output (`|GetArrayItem` (`self.scenesArray`) (`self.currentPlatformIndex`)))
  (`/Engine/EditorBlueprintResources/StandardMacros.IsValid` _output
    (:`Is Valid`
      (bind _output_get (set `self.currentPlatformLocation` (`SceneComponent.K2_GetComponentLocation` _output)))
      (bind _output_get_2 (set `self.currentPlatformRot` (`SceneComponent.K2_GetComponentRotation` (`SceneComponent.GetChildComponent` _output 0))))
      (bind (_direction _newtrack_0) (`Timeline|Timeline_SetPlatform` :!via `PlayFromStart`)
        (:`Update`
          (`SceneComponent.K2_SetWorldLocation` _output (`KismetMathLibrary.VLerp` _output_get (`SceneComponent.K2_GetComponentLocation` (`self.SceneObjective`)) _newtrack_0) false true)
          (`SceneComponent.K2_SetWorldRotation` (`SceneComponent.GetChildComponent` _output 0) (`KismetMathLibrary.RLerp` _output_get_2 (struct) _newtrack_0) false false))
        (:`Finished`
          (`/Engine/EditorBlueprintResources/StandardMacros.IncrementInt` (`self.currentPlatformIndex`)
            (:`  `
              (`self.MovePlatform`))))))))

(event `/Game/Blueprints/Interface_Platform.SetPlatform`
  (`/Engine/EditorBlueprintResources/StandardMacros.DoOnce` false
    (:`Completed`
      (`GameplayStatics.PlaySound2D` "/Game/Audio/SFX/Capacity/Revealer/S_Reveal.S_Reveal" 1.0 1.0 0.0 null null)
      (`self.MovePlatform`))))

(fn `UserConstructionScript`)