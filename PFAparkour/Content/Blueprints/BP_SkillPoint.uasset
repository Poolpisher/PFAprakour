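; Collectible skill point orb that grants skill points when the first-person character interacts with it.
; Box overlap registers the orb as the character's interact target and shows a HUD prompt.
; Interacting once disables collision, plays a collect montage and lerps the sphere to the hand socket before attaching it.
; DestroyOrb, exposed through the character's SkillOrbRef, adds points to the game instance, shows a notification and triggers the explosion effect.
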(event `self.Box.OnComponentBeginOverlap`
  (params (OverlappedComponent :type "PrimitiveComponent Object Reference") (OtherActor :type "Actor Object Reference") (OtherComp :type "PrimitiveComponent Object Reference") (OtherBodyIndex :type Integer) (bFromSweep :type Boolean) (SweepResult :type "HitResult Structure (by ref)"))
  (if (`self.CanInteract`)
    (bind _asbp_first_person_character (cast `/Game/FirstPerson/Blueprints/BP_FirstPersonCharacter` OtherActor))
    (set `/Game/FirstPerson/Blueprints/BP_FirstPersonCharacter.objectToInteractWith` self _asbp_first_person_character)
    (bind _returnvalue (`|CreateWidget` "/Game/Widget/W_Interact.W_Interact_C"))
    (bind _output_get (set `self.interactWidgetRef` _returnvalue))
    (`PanelWidget.AddChild` (`/Game/Widget/W_Main.BorderNotification` (`/Game/FirstPerson/Blueprints/BP_FirstPersonCharacter.mainHUD` _asbp_first_person_character)) _output_get)))

(event `self.Box.OnComponentEndOverlap`
  (params (OverlappedComponent :type "PrimitiveComponent Object Reference") (OtherActor :type "Actor Object Reference") (OtherComp :type "PrimitiveComponent Object Reference") (OtherBodyIndex :type Integer))
  (bind _asbp_first_person_character (cast `/Game/FirstPerson/Blueprints/BP_FirstPersonCharacter` OtherActor))
  (`/Game/Widget/W_Interact.DestroyIndic` (`self.interactWidgetRef`))
  (if (== (`/Game/FirstPerson/Blueprints/BP_FirstPersonCharacter.objectToInteractWith` _asbp_first_person_character) self)
    (set `/Game/FirstPerson/Blueprints/BP_FirstPersonCharacter.objectToInteractWith` null _asbp_first_person_character)))

(event `/Game/Blueprints/Interface_Interractible.Interract`
  (`/Engine/EditorBlueprintResources/StandardMacros.DoOnce` false
    (:`Completed`
      (set `self.CanInteract` false)
      (`|ExecutionSequence`
        (:`then_0`
          (`PrimitiveComponent.SetCollisionEnabled` (`self.Box`) "NoCollision"))
        (:`then_1`
          (bind _ascustom_game_instance (cast `/Game/CustomGameInstance` (`GameplayStatics.GetGameInstance`)))
          (bind _asbp_first_person_character (cast `/Game/FirstPerson/Blueprints/BP_FirstPersonCharacter` (`GameplayStatics.GetPlayerCharacter` 0)))
          (`TimelineComponent.Stop` (`self.MovementTimeline`))
          (set `/Game/FirstPerson/Blueprints/BP_FirstPersonCharacter.SkillOrbRef` self _asbp_first_person_character)
          (bind _firstpersonmesh (`/Game/FirstPerson/Blueprints/BP_FirstPersonCharacter.FirstPersonMesh` _asbp_first_person_character))
          (`|PlayMontage` _firstpersonmesh "/Game/FirstPersonArms/ParkourCharacter/MainCharacter/Animations/AM_CollectSkillOrb.AM_CollectSkillOrb"
            (:`then`
              (bind _output_get (set `self.BaseSphereLoc` (`SceneComponent.K2_GetComponentLocation` (`self.Sphere`))))
              (bind (_direction _lepr) (`Timeline|MoveSphereToHand` :!via `PlayFromStart`)
                (:`Update`
                  (`SceneComponent.K2_SetWorldLocation` (`self.Sphere`) (`KismetMathLibrary.VLerp` _output_get (`SceneComponent.GetSocketLocation` _firstpersonmesh "SkillSphere_socket") _lepr) false false))
                (:`Finished`
                  (`SceneComponent.K2_AttachToComponent` (`self.Sphere`) _firstpersonmesh "SkillSphere_socket" "SnapToTarget" "SnapToTarget" "KeepWorld" true))))))))))

(event `DestroyOrb`
  (`ActorComponent.K2_DestroyComponent` (`self.Sphere`))
  (`ActorComponent.K2_DestroyComponent` (`self.PointLight`))
  (set `/Game/CustomGameInstance.skillPoints` (+ (`/Game/CustomGameInstance.skillPoints` (stale `/Game/Blueprints/Interface_Interractible.Interract` _ascustom_game_instance)) (`self.skillPointToGive`)) (stale `/Game/Blueprints/Interface_Interractible.Interract` _ascustom_game_instance))
  (`/Game/Widget/W_Main.SetNotification` (`/Game/FirstPerson/Blueprints/BP_FirstPersonCharacter.mainHUD` (stale `/Game/Blueprints/Interface_Interractible.Interract` _asbp_first_person_character)) "/Game/Widget/W_SkillPoint_ObtentionNotify.W_SkillPoint_ObtentionNotify_C")
  (`ActorComponent.Activate` (`self.SphereCrackExplode`) true))

(fn `UserConstructionScript`)